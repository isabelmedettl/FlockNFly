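; BP_SpectatorCamera is an AI test camera that sends clicked world locations to a third-person character.
; Left click runs a persistent debug-drawn Visibility line trace from the actor toward the aim forward vector times TraceDistance, an end point not offset by actor location.
; The hit location, or that end point on a miss, goes to LineTraced on the first BP_ThirdPersonCharacter found and is marked with a debug sphere.
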(event `Key|LeftMouseButton`
  (params (Key :type "Key Structure"))
  (bind _returnvalue (* (`KismetMathLibrary.GetForwardVector` (`self.GetBaseAimRotation`)) (`self.TraceDistance`)))
  (:`Pressed`
    (bind (_outhit _returnvalue_2) (`KismetSystemLibrary.LineTraceSingle` :`Start` (`self.K2_GetActorLocation`) :`End` _returnvalue :`TraceChannel` "TraceTypeQuery1" :`DrawDebugType` "Persistent"))
    (if _returnvalue_2
      (bind _outactors (`GameplayStatics.GetAllActorsOfClass` "/Game/ThirdPerson/Blueprints/BP_ThirdPersonCharacter.BP_ThirdPersonCharacter_C"))
      (bind (_bblockinghit _binitialoverlap _time _distance _location) (`GameplayStatics.BreakHitResult` _outhit))
      (`/Game/ThirdPerson/Blueprints/BP_ThirdPersonCharacter.LineTraced` (`|GetArrayItem` _outactors) _location)
      (`KismetSystemLibrary.DrawDebugSphere` _location 30.0 30 (struct :`R` 1.0 :`A` 1.0) 10.0)
      (else
        (bind _outactors_2 (`GameplayStatics.GetAllActorsOfClass` "/Game/ThirdPerson/Blueprints/BP_ThirdPersonCharacter.BP_ThirdPersonCharacter_C"))
        (`/Game/ThirdPerson/Blueprints/BP_ThirdPersonCharacter.LineTraced` (`|GetArrayItem` _outactors_2) _returnvalue)
        (`KismetSystemLibrary.DrawDebugSphere` _returnvalue 30.0 30 (struct :`R` 1.0 :`A` 1.0) 10.0)))))

(fn `UserConstructionScript`)